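; BP_BaseWeapon is the base weapon actor for the combat system, defining what happens when a weapon is equipped.
; Its OnEquipped override marks it equipped, casts the owner to BP_CombatCharacter, and attaches to the hand socket or the attach socket depending on whether combat is enabled.
; It then registers itself as the character's main weapon and messages the mesh's anim instance with its combat type, without running the parent OnEquipped.
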(fn `OnEquipped`
  (`self.SetIsEquipped` true)
  (bind _asbp_combat_character (cast `/Game/CombatSystem/Blueprints/BP_CombatCharacter` (`self.GetOwner`)))
  (`self.AttachActor` (select `bool` (`/Game/CombatSystem/Blueprints/BP_CombatCharacter.IsCombatEnabled?` _asbp_combat_character) :`false` (`self.Attach Socket Name`) :`true` (`self.HandSocketName`)))
  (`/Game/CombatSystem/Blueprints/BP_CombatCharacter.SetMainWeapon` _asbp_combat_character self)
  (message `/Game/CombatSystem/Blueprints/Interfaces/AnimInstance_BPI.UpdateCombatType` (`SkeletalMeshComponent.GetAnimInstance` (`Character.Mesh` _asbp_combat_character)) (`self.CombatType`)))

(fn `UserConstructionScript`
  (`parent.UserConstructionScript`))